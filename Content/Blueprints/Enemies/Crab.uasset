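; Crab enemy that paces sideways along its local Y axis and sometimes jumps, with movement halted while paused.
; Tick reads a looping direction array, advancing every two seconds of walking and then rolling a random chance to jump.
; On BeginPlay it adds to its base speed, or zeroes it when DontMove is set, and spawns a shield or rings for its invincibility level.
; Those protective objects update every Tick to follow its location but not its rotation.
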(event `self.ReceiveBeginPlay`
  (`parent.ReceiveBeginPlay`)
  (set `self.Speed` (+ (`self.Speed`) 170.0))
  (if (`self.DontMove`)
    (set `self.Speed` 0.0))
  (`self.SetUpInvincibilityObjects`))

(event `self.ReceiveTick`
  (params (DeltaSeconds :type "Float (single-precision)"))
  (`self.Update Invincibility Objects` false)
  (if (`self.Unpaused`)
    ;[1 1 1] Decide which direction to walk to now
    (if (== (`|GetArrayItem` (`self.MovementDirectionArray`) (`self.CurrentMovementDirectionArrayIndex`)) 1)
      (set `self.WalkDirection` -1.0)
      (else
        (set `self.WalkDirection` 1.0)))
    (`self.K2_AddActorLocalOffset` (`KismetMathLibrary.MakeVector` 0.0 (* (`self.Speed`) (`GameplayStatics.GetWorldDeltaSeconds`) (`self.WalkDirection`))))
    ;[1 1 1] Has walked enough in one direction: move onto next direction stored in the array
    (bind _output_get (set `self.TimeWalked` (+ (`self.TimeWalked`) (`GameplayStatics.GetWorldDeltaSeconds`))))
    (if (>= _output_get 2.0)
      (if (== (`self.CurrentMovementDirectionArrayIndex`) (- (`KismetArrayLibrary.Array_Length` (`self.MovementDirectionArray`)) 1))
        (set `self.CurrentMovementDirectionArrayIndex` 0)
        (else
          (`/Engine/EditorBlueprintResources/StandardMacros.IncrementInt` (`self.CurrentMovementDirectionArrayIndex`)
            (:`  `
              _))))
      (set `self.TimeWalked` 0.0)
      (`self.ThrustUpwards` (`self.ChanceOfUpwardsThrust`)))))

(fn `Pause`
  (`parent.Pause`)
  (set `self.Unpaused` false))

(fn `SetUpInvincibilityObjects`
  (if (`self.HasInvincibilityLevel1`)
    (bind _returnvalue (`|SpawnActorFromClass` "/Game/Blueprints/Other/EnemyShield2x.EnemyShield2x_C" (`self.GetTransform`) "Undefined" "OverrideRootScale" null null))
    (set `/Game/Blueprints/Other/EnemyShield2x.Speed` (* (`/Game/Blueprints/Other/EnemyShield2x.Speed` _returnvalue) 1.5) _returnvalue)
    (set `self.Shield` _returnvalue)
    (elif (`self.HasInvincibilityLevel2`)
      (bind _returnvalue_2 (`|SpawnActorFromClass` "/Game/Blueprints/Other/EnemyRing.EnemyRing_C" (`KismetMathLibrary.MakeTransform` (`self.K2_GetActorLocation`) (struct) (1.0 2.2 2.2)) "Undefined" "OverrideRootScale" null null))
      (set `self.Ring1` _returnvalue_2)
      (elif (`self.HasInvincibilityLevel3`)
        (`|ExecutionSequence`
          (:`then_0`
            (bind _returnvalue_3 (`|SpawnActorFromClass` "/Game/Blueprints/Other/EnemyRing.EnemyRing_C" (`KismetMathLibrary.MakeTransform` (`self.K2_GetActorLocation`) (struct) (0.3 2.4 2.2)) "Undefined" "OverrideRootScale" null null))
            (set `/Game/Blueprints/Other/EnemyRing.Speed` 160.0 _returnvalue_3)
            (set `self.Ring1` _returnvalue_3))
          (:`then_1`
            (bind _returnvalue_4 (`|SpawnActorFromClass` "/Game/Blueprints/Other/EnemyRing.EnemyRing_C" (`KismetMathLibrary.MakeTransform` (`self.K2_GetActorLocation`) (struct) (0.3 2.4 2.2)) "Undefined" "OverrideRootScale" null null))
            (set `/Game/Blueprints/Other/EnemyRing.Speed` 160.0 _returnvalue_4)
            (bind _output_get (set `self.Ring2` _returnvalue_4))
            (`self.K2_AddActorLocalRotation` _output_get (struct :`Yaw` 90.0) false false)))))))

(fn `Unpause`
  (`parent.Unpause`)
  (set `self.Unpaused` true))

(fn `UserConstructionScript`
  (`parent.UserConstructionScript`))