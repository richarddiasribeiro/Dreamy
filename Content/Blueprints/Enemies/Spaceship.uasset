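; Enemy spaceship that spins its mesh and flies a looping, pausable patrol path.
; Tick moves it forward and every two seconds applies the next step of a direction array (straight or a 90-degree left or right yaw), wrapping the index.
; BeginPlay inverts the configured Speed against a constant.
; PullPlayerUp toggles the player's abduction flag but is not called here; its walk-speed and jump changes are disconnected.
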(event `self.ReceiveBeginPlay`
  (`parent.ReceiveBeginPlay`)
  (set `self.Speed` (/ 100000.0 (`self.Speed`))))

(event `self.ReceiveTick`
  (params (DeltaSeconds :type "Float (single-precision)"))
  (if (`self.Unpaused`)
    ;[1 1 1] Spin the mesh
    (`SceneComponent.K2_AddLocalRotation` (`self.StaticMesh`) (`KismetMathLibrary.MakeRotator` 0.0 0.0 (* DeltaSeconds 270.0)) false false)
    ;[1 1 1] Fly forward
    (`self.K2_AddActorLocalOffset` (`KismetMathLibrary.MakeVector` (* (`self.Speed`) (`GameplayStatics.GetWorldDeltaSeconds`))))
    ;[1 1 1] Has flight enough in one direction: move onto next direction stored in the array
    (bind _output_get (set `self.TimeFlight` (+ (`self.TimeFlight`) (`GameplayStatics.GetWorldDeltaSeconds`))))
    (if (>= _output_get 2.0)
      (switch `int` (`|GetArrayItem` (`self.MovementDirectionArray`) (`self.CurrentMovementDirectionArrayIndex`))
        (:`0`
          _)
        (:`1`
          (`self.K2_AddActorLocalRotation` (struct :`Yaw` -90.0)))
        (:`2`
          (`self.K2_AddActorLocalRotation` (struct :`Yaw` 90.0))))
      (if (== (`self.CurrentMovementDirectionArrayIndex`) (- (`KismetArrayLibrary.Array_Length` (`self.MovementDirectionArray`)) 1))
        (set `self.CurrentMovementDirectionArrayIndex` 0)
        (else
          (`/Engine/EditorBlueprintResources/StandardMacros.IncrementInt` (`self.CurrentMovementDirectionArrayIndex`)
            (:`  `
              _))))
      (set `self.TimeFlight` 0.0))))

(fn `Pause`
  (`parent.Pause`)
  (set `self.Unpaused` false))

(fn `Unpause`
  (`parent.Unpause`)
  (set `self.Unpaused` true))

(fn `UserConstructionScript`
  (`parent.UserConstructionScript`))