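; Penguin enemy that patrols back and forth, moving forward up to a maximum offset before turning around.
; Tick accumulates walked distance, then a DoOnce-gated sequence pitches it 90 degrees, waits, rotates it around and resets.
; BeginPlay derives the pause inversely from Speed before multiplying Speed for movement.
; A separate FollowPlayer graph issues AIMoveTo toward the player's location, but nothing here calls it.
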(event `self.ReceiveBeginPlay`
  (`parent.ReceiveBeginPlay`)
  (set `self.StandUpDelay` (/ 100.0 (`self.Speed`)))
  (set `self.Speed` (* (`self.Speed`) 6.0)))

(event `self.ReceiveTick`
  (params (DeltaSeconds :type "Float (single-precision)"))
  (bind _returnvalue (* DeltaSeconds (`self.Speed`)))
  ;[1 1 1] Make the enemy move forward untill a certain distance, wait and then turn around
  (if (>= (`self.WalkedOffset`) (`self.MaxOffset`))
    (`/Engine/EditorBlueprintResources/StandardMacros.DoOnce` false :!label _label
      (:`Completed`
        (`self.K2_AddActorLocalRotation` (`KismetMathLibrary.MakeRotator` 0.0 90.0))
        (`KismetSystemLibrary.Delay` (`self.StandUpDelay`))
        (`self.K2_AddActorLocalRotation` (`KismetMathLibrary.MakeRotator` 0.0 90.0 180.0))
        (set `self.WalkedOffset` 0.0)
        (goto _label :!via `Reset`)))
    (else
      (`self.K2_AddActorLocalOffset` (`KismetMathLibrary.MakeVector` _returnvalue))
      (set `self.WalkedOffset` (+ (`self.WalkedOffset`) _returnvalue)))))

(fn `UserConstructionScript`
  (`parent.UserConstructionScript`))