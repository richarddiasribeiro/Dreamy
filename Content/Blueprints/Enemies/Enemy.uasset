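; Enemy actor that supplies player detection, chase and pause helpers, with speed scaled to the game instance's current level at BeginPlay.
; Sphere and downward-offset capsule traces report whether the player is near or beneath it.
; FollowPlayer turns toward the player, optionally by yaw only, and moves forward, while a line trace drives simulated gravity.
; Tick is disabled and nothing here calls these functions; pausing zeroes time dilation and stops the mesh animation.
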(event `self.ReceiveBeginPlay`
  (bind _returnvalue (`GameplayStatics.GetActorOfClass` "/Game/Blueprints/ThirdPersonCharacter.ThirdPersonCharacter_C"))
  (set `self.Player` _returnvalue)
  ;[1 1 1] Progressive enemy speed based on the player's progression (current level)
  (bind _asnew_platform_game_instance (cast `/Game/Blueprints/NewPlatformGameInstance` (`GameplayStatics.GetGameInstance`)))
  (set `self.Speed` (+ 100.0 (* (`/Game/Blueprints/NewPlatformGameInstance.CurrentLevel` _asnew_platform_game_instance) 3.75))))

(event `self.ReceiveActorBeginOverlap`
  (params (OtherActor :type "Actor Object Reference")))

(event `DestroySelf`
  (`self.K2_DestroyActor`))

(fn `FollowPlayer`
  (params (LookOnlyInTheZAxis :type Boolean))
  (bind (_returnvalue_roll _returnvalue_pitch) (`KismetMathLibrary.BreakRotator` (`self.K2_GetActorRotation`)))
  (bind (_returnvalue_roll_2 _returnvalue_pitch_2 _returnvalue_yaw) (`KismetMathLibrary.BreakRotator` (`KismetMathLibrary.FindLookAtRotation` (`self.K2_GetActorLocation`) (`self.K2_GetActorLocation` (`self.Player`)))))
  (if LookOnlyInTheZAxis
    (`self.K2_SetActorRotation` (`KismetMathLibrary.MakeRotator` _returnvalue_roll _returnvalue_pitch _returnvalue_yaw))
    (else
      (`SceneComponent.K2_SetWorldRotation` (`self.CapsuleComponent`) (`KismetMathLibrary.FindLookAtRotation` (`self.K2_GetActorLocation`) (`self.K2_GetActorLocation` (`self.Player`))) false false)))
  (`self.K2_AddActorLocalOffset` (`KismetMathLibrary.MakeVector` (* (`self.Speed`) (`GameplayStatics.GetWorldDeltaSeconds`)))))

(fn `IsPlayerBeneath`
  (returns (Result :type Boolean))
  (bind (_returnvalue_x _returnvalue_y _returnvalue_z) (`KismetMathLibrary.BreakVector` (`self.K2_GetActorLocation`)))
  (bind _returnvalue (`KismetMathLibrary.MakeVector` _returnvalue_x _returnvalue_y (+ (- _returnvalue_z (`self.CapsuleTraceHalfHeight`)) 75.0)))
  (bind (_outhit _returnvalue_2) (`KismetSystemLibrary.CapsuleTraceSingleForObjects` _returnvalue _returnvalue (`self.CapsuleTraceRadius`) (`self.CapsuleTraceHalfHeight`) (`self.Object Types`)))
  (cast `/Game/Blueprints/ThirdPersonCharacter` (`.HitActor` (`GameplayStatics.BreakHitResult` _outhit))
    (:`then`
      (if _returnvalue_2
        (return true)
        (else
          _)))
    (:`CastFailed`
      _))
  (return false))

(fn `IsPlayerNear`
  (returns (Result :type Boolean))
  (bind _returnvalue (`self.K2_GetActorLocation`))
  (bind (_outhit _returnvalue_2) (`KismetSystemLibrary.SphereTraceSingleForObjects` _returnvalue _returnvalue (`self.SphereTraceRadius`) (`self.Object Types`)))
  (cast `/Game/Blueprints/ThirdPersonCharacter` (`.HitActor` (`GameplayStatics.BreakHitResult` _outhit))
    (:`then`
      (if _returnvalue_2
        (return true)
        (else
          _)))
    (:`CastFailed`
      _))
  (return false))

(fn `Pause`
  (set `self.CustomTimeDilation` 0.0)
  (`SkeletalMeshComponent.Stop` (`self.Mesh`)))

(fn `SimulateGravityInTheZAxis`
  (bind (_returnvalue_x _returnvalue_y _returnvalue_z) (`KismetMathLibrary.BreakVector` (`self.K2_GetActorLocation`)))
  (bind (_outhit _returnvalue) (`KismetSystemLibrary.LineTraceSingle` (`self.K2_GetActorLocation`) (`KismetMathLibrary.MakeVector` _returnvalue_x _returnvalue_y (- _returnvalue_z (`self.MinimumDistanceFromGround`))) "TraceTypeQuery1"))
  (if (not _returnvalue)
    (`self.K2_AddActorLocalOffset` (`KismetMathLibrary.MakeVector` 0.0 0.0 (* (`GameplayStatics.GetWorldDeltaSeconds`) -500.0)))))

(fn `Unpause`
  (set `self.CustomTimeDilation` 1.0)
  (`SkeletalMeshComponent.Play` (`self.Mesh`) true))

(fn `UserConstructionScript`)