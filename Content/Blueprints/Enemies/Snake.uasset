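; Snake enemy that patrols back and forth and chases the player when nearby, built on a parent enemy class.
; BeginPlay raises the inherited speed and scales the movement component's max walk speed from it.
; Tick moves it forward by direct local offsets, flipping yaw at the distance limit.
; While IsPlayerNear is true, FollowPlayer also issues AIMoveTo toward the player's full location every frame, without pausing the patrol.
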(event `self.ReceiveBeginPlay`
  (`parent.ReceiveBeginPlay`)
  (set `self.Speed` (+ (`self.Speed`) 160.0))
  (set `CharacterMovementComponent.MaxWalkSpeed` (* (`self.Speed`) 1.5) (`self.CharacterMovement`)))

(event `self.ReceiveTick`
  (params (DeltaSeconds :type "Float (single-precision)"))
  (bind _returnvalue (* DeltaSeconds (`self.Speed`)))
  ;[1 1 1] Make the enemy move forward untill a certain distance and then turn around
  (if (>= (`self.WalkedOffset`) (`self.MaxOffset`))
    (`self.K2_AddActorLocalRotation` (`KismetMathLibrary.MakeRotator` 0.0 0.0 180.0))
    (set `self.WalkedOffset` 0.0)
    (else
      (`self.K2_AddActorLocalOffset` (`KismetMathLibrary.MakeVector` _returnvalue))
      (set `self.WalkedOffset` (+ (`self.WalkedOffset`) _returnvalue))))
  ;[1 1 1] Chase the player
  (bind _result (`self.IsPlayerNear`))
  (if _result
    (`self.FollowPlayer`)))

(fn `UserConstructionScript`
  (`parent.UserConstructionScript`))