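; Anchor enemy that chases the player and plays its anchor animation when horizontally close.
; BeginPlay runs the parent logic, doubles Speed and trace radius, then sets walk speed to twice the doubled Speed.
; Tick issues AIMoveTo while IsPlayerNear holds, and separately plays the slowed, non-looping animation within MinimumDistanceToDrop unless one is playing.
; The DropAnchor macro is not used in the event graph.
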(event `self.ReceiveBeginPlay`
  (`parent.ReceiveBeginPlay`)
  (set `self.Speed` (* (`self.Speed`) 2.0))
  (set `self.SphereTraceRadius` (* (`self.SphereTraceRadius`) 2.0))
  (set `CharacterMovementComponent.MaxWalkSpeed` (* (`self.Speed`) 2.0) (`self.CharacterMovement`)))

(event `self.ReceiveTick`
  (params (DeltaSeconds :type "Float (single-precision)"))
  (bind _mesh (`self.Mesh`))
  (bind _result (`self.IsPlayerNear`))
  (if _result
    (`self.FollowPlayerMacro`))
  (if (and (< (`self.GetHorizontalDistanceTo` (`self.Player`)) (`self.MinimumDistanceToDrop`)) (not (`SkeletalMeshComponent.IsPlaying` (`self.Mesh`))))
    (`SkeletalMeshComponent.SetPlayRate` _mesh 0.75)
    (`SkeletalMeshComponent.PlayAnimation` _mesh "/Game/MeshesAndAnimations/Enemies/Anchor_Anim.Anchor_Anim" false)))

(fn `UserConstructionScript`
  (`parent.UserConstructionScript`))