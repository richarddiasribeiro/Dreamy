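; Bee enemy Blueprint that follows the player when the player is near, built on a parent class.
; On BeginPlay it triples the inherited speed, doubles the sphere trace radius and sets movement gravity to zero so it is not pulled down.
; Each Tick it calls IsPlayerNear and, when that returns true, calls FollowPlayer.
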(event `self.ReceiveBeginPlay`
  (`parent.ReceiveBeginPlay`)
  (set `self.Speed` (* (`self.Speed`) 3.0))
  (set `self.SphereTraceRadius` (* (`self.SphereTraceRadius`) 2.0))
  (set `CharacterMovementComponent.GravityScale` 0.0 (`self.CharacterMovement`)))

(event `self.ReceiveTick`
  (params (DeltaSeconds :type "Float (single-precision)"))
  (bind _result (`self.IsPlayerNear`))
  (if _result
    (`self.FollowPlayer` false)))

(fn `UserConstructionScript`
  (`parent.UserConstructionScript`))