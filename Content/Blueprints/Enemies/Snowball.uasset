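; Snowball enemy that rolls forward along its local X axis and loops back to its spawn point.
; Tick spins the mesh and moves the actor at a speed quadrupled on BeginPlay, growing the capsule as it travels.
; At MaxOffset, helper graphs play black hole Niagara effects at both ends around a briefly delayed teleport that resets distance and scale.
; A FollowPlayer AI move graph exists but is not called here.
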(event `self.ReceiveBeginPlay`
  (`parent.ReceiveBeginPlay`)
  (set `self.Speed` (* (`self.Speed`) 4.0))
  (set `self.InitialLocation` (`self.K2_GetActorLocation`)))

(event `self.ReceiveTick`
  (params (DeltaSeconds :type "Float (single-precision)"))
  (bind _blackholeniagaraparticlesystemstart (`self.BlackHoleNiagaraParticleSystemStart`))
  (bind _blackholeniagaraparticlesystemend (`self.BlackHoleNiagaraParticleSystemEnd`))
  (bind _returnvalue (* DeltaSeconds (`self.Speed`)))
  ;[1 1 1] Spin the mesh
  (`SceneComponent.K2_AddLocalRotation` (`self.StaticMesh`) (`KismetMathLibrary.MakeRotator` 0.0 (* DeltaSeconds (`self.Speed`) -1.0)) false false)
  ;[1 1 1] Make the enemy move forward untill a certain distance and then go back to its initial position
  (if (>= (`self.WalkedOffset`) (`self.MaxOffset`))
    (`SceneComponent.K2_SetWorldLocation` _blackholeniagaraparticlesystemstart (`self.K2_GetActorLocation`) false false)
    (`ActorComponent.Activate` _blackholeniagaraparticlesystemstart true)
    (`KismetSystemLibrary.Delay` 0.1)
    (`self.K2_SetActorLocation` (`self.InitialLocation`))
    (set `self.WalkedOffset` 0.0)
    ;[1 1 1] Reset the capsule's size
    (`SceneComponent.SetWorldScale3D` (`self.CapsuleComponent`) (1.0 1.0 1.0))
    (`SceneComponent.K2_SetWorldLocation` _blackholeniagaraparticlesystemend (`self.InitialLocation`) false false)
    (`ActorComponent.Activate` _blackholeniagaraparticlesystemend true)
    (else
      (`self.K2_AddActorLocalOffset` (`KismetMathLibrary.MakeVector` _returnvalue))
      (set `self.WalkedOffset` (+ (`self.WalkedOffset`) _returnvalue))
      ;[1 1 1] Gradually increase the capsule's size
      (`SceneComponent.SetWorldScale3D` (`self.CapsuleComponent`) (+ (`SceneComponent.K2_GetComponentScale` (`self.CapsuleComponent`)) (/ _returnvalue 50.0))))))

(fn `UserConstructionScript`
  (`parent.UserConstructionScript`))