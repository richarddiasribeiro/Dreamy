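; Clam enemy that lunges forward along its local X axis when its PawnSensing component sees a pawn.
; On BeginPlay it runs the parent logic and doubles Speed.
; A sighting telegraphs the attack by freezing the mesh animation for a Speed-based delay, then raises the play rate.
; A Delay-driven loop applies stepped local offsets scaled by Speed and frame time until Steps reaches MaxSteps, then resets the counter.
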(event `self.ReceiveBeginPlay`
  (`parent.ReceiveBeginPlay`)
  (set `self.Speed` (* (`self.Speed`) 2.0)))

(event `self.ReceiveTick`
  (params (DeltaSeconds :type "Float (single-precision)")))

(event `self.PawnSensing.OnSeePawn`
  (params (Pawn :type "Pawn Object Reference"))
  (bind _steps (`self.Steps`))
  ;[1 1 1] Tell the attack
  (`SkeletalMeshComponent.SetPlayRate` (`self.Mesh`) 0.0)
  (`KismetSystemLibrary.Delay` (/ (`self.Speed`) 400.0))
  (`SkeletalMeshComponent.SetPlayRate` (`self.Mesh`) 4.0)
  ;[1 1 1] Attack
  (`self.K2_AddActorLocalOffset` (`KismetMathLibrary.MakeVector` (* (`self.Speed`) (`GameplayStatics.GetWorldDeltaSeconds`) 50.0)) :!label _label)
  (`KismetSystemLibrary.Delay` 0.05)
  (if (< _steps (`self.MaxSteps`))
    (`/Engine/EditorBlueprintResources/StandardMacros.IncrementInt` _steps
      (:`  `
        (goto _label)))
    (else
      (set `self.Steps` 0))))

(fn `UserConstructionScript`
  (`parent.UserConstructionScript`))