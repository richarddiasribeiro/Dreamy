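; Frog enemy, a child Blueprint that jumps and uses AI MoveTo to chase the player whenever they are near.
; BeginPlay multiplies inherited speed and sphere trace radius, then spawns a shield, one ring or two crossed rings according to invincibility flags.
; Tick keeps these objects on the frog's location without following its rotation, and runs the proximity check that triggers the chase.
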(event `self.ReceiveBeginPlay`
  (`parent.ReceiveBeginPlay`)
  (set `self.Speed` (* (`self.Speed`) 2.5))
  (set `self.SphereTraceRadius` (* (`self.SphereTraceRadius`) 2.5))
  (`self.SetUpInvincibilityObjects`))

(event `self.ReceiveTick`
  (params (DeltaSeconds :type "Float (single-precision)"))
  (`self.Update Invincibility Objects` false)
  (bind _result (`self.IsPlayerNear`))
  (if _result
    (`self.Jump`)
    (`self.FollowPlayer` false)))

(fn `DoFrogChase`
  (params (ChaseForce :type "Float (double-precision)" :default 2000.0))
  (`self.Jump`))

(fn `SetUpInvincibilityObjects`
  (if (`self.HasInvincibilityLevel1`)
    (bind _returnvalue (`|SpawnActorFromClass` "/Game/Blueprints/Other/EnemyShield2x.EnemyShield2x_C" (`self.GetTransform`) "Undefined" "OverrideRootScale" null null))
    (set `self.Shield` _returnvalue)
    (elif (`self.HasInvincibilityLevel2`)
      (bind _returnvalue_2 (`|SpawnActorFromClass` "/Game/Blueprints/Other/EnemyRing.EnemyRing_C" (`KismetMathLibrary.MakeTransform` (`self.K2_GetActorLocation`) (struct) (1.0 2.0 2.0)) "Undefined" "OverrideRootScale" null null))
      (set `self.Ring1` _returnvalue_2)
      (elif (`self.HasInvincibilityLevel3`)
        (`|ExecutionSequence`
          (:`then_0`
            (bind _returnvalue_3 (`|SpawnActorFromClass` "/Game/Blueprints/Other/EnemyRing.EnemyRing_C" (`KismetMathLibrary.MakeTransform` (`self.K2_GetActorLocation`) (struct) (0.3 2.0 2.0)) "Undefined" "OverrideRootScale" null null))
            (set `/Game/Blueprints/Other/EnemyRing.Speed` 160.0 _returnvalue_3)
            (set `self.Ring1` _returnvalue_3))
          (:`then_1`
            (bind _returnvalue_4 (`|SpawnActorFromClass` "/Game/Blueprints/Other/EnemyRing.EnemyRing_C" (`KismetMathLibrary.MakeTransform` (`self.K2_GetActorLocation`) (struct) (0.3 2.0 2.0)) "Undefined" "OverrideRootScale" null null))
            (set `/Game/Blueprints/Other/EnemyRing.Speed` 160.0 _returnvalue_4)
            (bind _output_get (set `self.Ring2` _returnvalue_4))
            (`self.K2_AddActorLocalRotation` _output_get (struct :`Yaw` 90.0) false false)))))))

(fn `UserConstructionScript`
  (`parent.UserConstructionScript`))