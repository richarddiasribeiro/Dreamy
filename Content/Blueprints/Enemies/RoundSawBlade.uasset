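; Round saw blade enemy that travels along its local X axis while spinning, curving its path when given a Z-axis rotation speed.
; MoveClockwise sets the direction sign applied each Tick to mesh spin, actor yaw and movement.
; On BeginPlay it scales up Speed and spawns a shield, one ring or two crossed rings by invincibility level.
; These follow its location without rotation, reversing their speed when the yaw rate is positive.
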(event `self.ReceiveBeginPlay`
  (`parent.ReceiveBeginPlay`)
  (set `self.Speed` (* (`self.Speed`) 6.0))
  (set `self.RotationDirectionFloat` (* (`self.Speed`) 0.8))
  (if (`self.MoveClockwise`)
    (set `self.RotationDirectionFloat` 1.0)
    (else
      (set `self.RotationDirectionFloat` -1.0)))
  (`self.SetUpInvincibilityObjects`))

(event `self.ReceiveTick`
  (params (DeltaSeconds :type "Float (single-precision)"))
  (`self.Update Invincibility Objects` false)
  ;[1 1 1] Spin the mesh
  (`SceneComponent.K2_AddLocalRotation` (`self.StaticMesh`) (`KismetMathLibrary.MakeRotator` 0.0 (* (`self.Speed`) (`self.RotationDirectionFloat`) -1.0 DeltaSeconds)) false false)
  ;[1 1 1] Move actor
  (`self.K2_AddActorLocalRotation` (`KismetMathLibrary.MakeRotator` 0.0 0.0 (* (`self.SawZAxisRotationSpeed`) (`self.RotationDirectionFloat`) DeltaSeconds)))
  (`self.K2_AddActorLocalOffset` (`KismetMathLibrary.MakeVector` (* (`self.Speed`) (`self.RotationDirectionFloat`) DeltaSeconds))))

(fn `InvertRingRotBasedOnEnemyRot`
  (params (Ring :type "/Game/Blueprints/Other/EnemyRing Object Reference"))
  (if (> (`self.SawZAxisRotationSpeed`) 0.0)
    (set `/Game/Blueprints/Other/EnemyRing.Speed` (* (`/Game/Blueprints/Other/EnemyRing.Speed` Ring) -1.0) Ring)))

(fn `InvertShieldRotBasedOnEnemyRot`
  (params (Shield :type "/Game/Blueprints/Other/EnemyShield2x Object Reference"))
  (if (> (`self.SawZAxisRotationSpeed`) 0.0)
    (set `/Game/Blueprints/Other/EnemyShield2x.Speed` (* (`/Game/Blueprints/Other/EnemyShield2x.Speed` Shield) -1.0) Shield)))

(fn `SetUpInvincibilityObjects`
  (if (`self.HasInvincibilityLevel1`)
    (bind _returnvalue (`|SpawnActorFromClass` "/Game/Blueprints/Other/EnemyShield2x.EnemyShield2x_C" (`KismetMathLibrary.MakeTransform` (`self.K2_GetActorLocation`) (struct) (1.2 1.2 1.2)) "Undefined" "OverrideRootScale" null null))
    (`self.InvertShieldRotBasedOnEnemyRot` _returnvalue)
    (set `self.Shield` _returnvalue)
    (elif (`self.HasInvincibilityLevel2`)
      (bind _returnvalue_2 (`|SpawnActorFromClass` "/Game/Blueprints/Other/EnemyRing.EnemyRing_C" (`KismetMathLibrary.MakeTransform` (`self.K2_GetActorLocation`) (struct) (1.0 2.0 2.0)) "Undefined" "OverrideRootScale" null null))
      (`self.InvertRingRotBasedOnEnemyRot` _returnvalue_2)
      (set `self.Ring1` _returnvalue_2)
      (elif (`self.HasInvincibilityLevel3`)
        (`|ExecutionSequence`
          (:`then_0`
            (bind _returnvalue_3 (`|SpawnActorFromClass` "/Game/Blueprints/Other/EnemyRing.EnemyRing_C" (`KismetMathLibrary.MakeTransform` (`self.K2_GetActorLocation`) (struct) (0.3 2.2 2.2)) "Undefined" "OverrideRootScale" null null))
            (set `/Game/Blueprints/Other/EnemyRing.Speed` 160.0 _returnvalue_3)
            (`self.InvertRingRotBasedOnEnemyRot` _returnvalue_3)
            (set `self.Ring1` _returnvalue_3))
          (:`then_1`
            (bind _returnvalue_4 (`|SpawnActorFromClass` "/Game/Blueprints/Other/EnemyRing.EnemyRing_C" (`KismetMathLibrary.MakeTransform` (`self.K2_GetActorLocation`) (struct) (0.3 2.2 2.2)) "Undefined" "OverrideRootScale" null null))
            (set `/Game/Blueprints/Other/EnemyRing.Speed` 160.0 _returnvalue_4)
            (`self.InvertRingRotBasedOnEnemyRot` _returnvalue_4)
            (bind _output_get (set `self.Ring2` _returnvalue_4))
            (`self.K2_AddActorLocalRotation` _output_get (struct :`Yaw` 90.0) false false)))))))

(fn `UserConstructionScript`
  (`parent.UserConstructionScript`))