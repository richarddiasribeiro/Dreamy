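; SpikeWreckingBall is an enemy Blueprint, with inherited character components, that acts as a continuously spinning hazard.
; On BeginPlay it runs the parent logic, raises Speed by a fixed amount, and destroys its Mesh and CharacterMovement components.
; Each Tick calls the parent, then adds local yaw scaled by Speed and delta time for frame-rate-independent rotation.
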(event `self.ReceiveBeginPlay`
  (`parent.ReceiveBeginPlay`)
  (set `self.Speed` (+ (`self.Speed`) 50.0))
  (`ActorComponent.K2_DestroyComponent` (`self.Mesh`))
  (`ActorComponent.K2_DestroyComponent` (`self.CharacterMovement`)))

(event `self.ReceiveTick`
  (params (DeltaSeconds :type "Float (single-precision)"))
  (`parent.ReceiveTick` DeltaSeconds)
  (`self.K2_AddActorLocalRotation` (`KismetMathLibrary.MakeRotator` 0.0 0.0 (* DeltaSeconds (`self.Speed`)))))

(fn `UserConstructionScript`
  (`parent.UserConstructionScript`))