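; Eagle enemy, a child Blueprint that boosts the inherited speed and flies continuously along its local forward axis while unpaused.
; EnemyRotationArray steers it: each entry's Origin serves as a turn rate and Target as the facing direction that advances to the next entry, looping.
; At BeginPlay it spawns a scaled, zero-speed ring for invincibility level 2 or 3, and updates invincibility objects each tick to follow its location and rotation.
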(event `self.ReceiveBeginPlay`
  (`parent.ReceiveBeginPlay`)
  ;[1 1 1] Override parent class' atributes
  (set `self.Speed` (* (`self.Speed`) 9.0))
  (`self.SetUpInvincibilityObjects`))

(event `self.ReceiveTick`
  (params (DeltaSeconds :type "Float (single-precision)"))
  (bind _output (`|GetArrayItem` (`self.EnemyRotationArray`) (`self.CurrentRotationSequenceArrayIndex`)))
  (bind (_output_origin _output_target) (break `/Game/Structs/EnemyRotation` (`|GetArrayItem` (`self.EnemyRotationArray`) (`self.CurrentRotationSequenceArrayIndex`))))
  (`self.Update Invincibility Objects` true)
  (if (`self.Unpaused`)
    (`self.K2_AddActorLocalOffset` (`KismetMathLibrary.MakeVector` (* (`self.Speed`) (`GameplayStatics.GetWorldDeltaSeconds`))))
    ;[1 1 1] Rotate according to the array
    (`self.K2_AddActorLocalRotation` (* (`KismetMathLibrary.MakeRotator` (.x (break `/Game/Structs/EnemyRotation` _output)) (.y (break `/Game/Structs/EnemyRotation` _output)) (.z (break `/Game/Structs/EnemyRotation` _output))) (`GameplayStatics.GetWorldDeltaSeconds`)))
    ;[1 1 1] Has flight enough towards one direction: move onto next direction stored in the array
    (if (== (`self.K2_GetActorRotation`) (`KismetMathLibrary.Conv_VectorToRotator` _output_target) :`ErrorTolerance` 0.1)
      (if (== (`self.CurrentRotationSequenceArrayIndex`) (- (`KismetArrayLibrary.Array_Length` (`self.EnemyRotationArray`)) 1))
        (set `self.CurrentRotationSequenceArrayIndex` 0)
        (else
          (`/Engine/EditorBlueprintResources/StandardMacros.IncrementInt` (`self.CurrentRotationSequenceArrayIndex`)))))))

(fn `InvertRingRotBasedOnEnemyRot`
  (params (Ring :type "/Game/Blueprints/Other/EnemyRing Object Reference"))
  (if (> (.z (break `/Game/Structs/EnemyRotation` (`|GetArrayItem` (`self.EnemyRotationArray`)))) 0.0)
    (set `/Game/Blueprints/Other/EnemyRing.Speed` (* (`/Game/Blueprints/Other/EnemyRing.Speed` Ring) -1.0) Ring)))

(fn `InvertShieldRotBasedOnEnemyRot`
  (params (Shield :type "/Game/Blueprints/Other/EnemyShield2x Object Reference"))
  (if (> (.z (break `/Game/Structs/EnemyRotation` (`|GetArrayItem` (`self.EnemyRotationArray`)))) 0.0)
    (set `/Game/Blueprints/Other/EnemyShield2x.Speed` (* (`/Game/Blueprints/Other/EnemyShield2x.Speed` Shield) -1.0) Shield)))

(fn `Pause`
  (`parent.Pause`)
  (set `self.Unpaused` false))

(fn `SetUpInvincibilityObjects`
  (if (`self.HasInvincibilityLevel1`)
    _
    (elif (`self.HasInvincibilityLevel2`)
      (bind _returnvalue (`|SpawnActorFromClass` "/Game/Blueprints/Other/EnemyRing.EnemyRing_C" (`KismetMathLibrary.MakeTransform` (`self.K2_GetActorLocation`) (struct) (1.0 2.2 2.2)) "Undefined" "OverrideRootScale" null null))
      (set `/Game/Blueprints/Other/EnemyRing.Speed` 0.0 _returnvalue)
      (`self.InvertRingRotBasedOnEnemyRot` _returnvalue)
      (set `self.Ring1` _returnvalue)
      (elif (`self.HasInvincibilityLevel3`)
        (bind _returnvalue_2 (`|SpawnActorFromClass` "/Game/Blueprints/Other/EnemyRing.EnemyRing_C" (`KismetMathLibrary.MakeTransform` (`self.K2_GetActorLocation`) (struct) (2.0 2.5 2.5)) "Undefined" "OverrideRootScale" null null))
        (set `/Game/Blueprints/Other/EnemyRing.Speed` 0.0 _returnvalue_2)
        (`self.InvertRingRotBasedOnEnemyRot` _returnvalue_2)
        (set `self.Ring1` _returnvalue_2)))))

(fn `Unpause`
  (`parent.Unpause`)
  (set `self.Unpaused` true))

(fn `UserConstructionScript`
  (`parent.UserConstructionScript`))