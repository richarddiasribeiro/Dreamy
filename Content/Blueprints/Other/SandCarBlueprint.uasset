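; SandCarBlueprint is an actor that travels forward and upward for a set time, then falls.
; Tick accumulates a timer and, until it passes TimeToStartFall, offsets the actor along local X and Z at Speed scaled by delta time.
; After that, the offset stops and each tick enables physics simulation on the StaticMesh, handing motion to the physics engine.
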(event `self.ReceiveTick`
  (params (DeltaSeconds :type "Float (single-precision)"))
  (bind _returnvalue (* (`self.Speed`) (`GameplayStatics.GetWorldDeltaSeconds`)))
  (set `self.Timer` (+ DeltaSeconds (`self.Timer`)))
  (if (> (`self.Timer`) (`self.TimeToStartFall`))
    ;[1 1 1] Start falling
    (`PrimitiveComponent.SetSimulatePhysics` (`self.StaticMesh`) true)
    (else
      ;[1 1 1] Move forward and upwards
      (`self.K2_AddActorLocalOffset` (`KismetMathLibrary.MakeVector` _returnvalue 0.0 _returnvalue)))))

(fn `UserConstructionScript`)