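; JigsawLevelPieceBase is a target spot in a jigsaw puzzle level that tracks whether its matching movable block is in place.
; Tick spins an arrow mesh and bobs it up and down as a marker.
; A box overlap with a JigsawLevelPieceMovableBlock of equal piece index sets the placed-correctly flag, while any end overlap clears it.
; Both changes make the level's JigsawPuzzleLevelBarrier recheck puzzle status.
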(event `self.ReceiveTick`
  (params (DeltaSeconds :type "Float (single-precision)"))
  (`SceneComponent.K2_AddLocalRotation` (`self.ArrowStaticMesh`) (`KismetMathLibrary.MakeRotator` 0.0 0.0 (* DeltaSeconds (`self.ArrowRotationSpeed`))) false false)
  (if (`self.MoveArrowUp`)
    (`SceneComponent.K2_AddLocalOffset` (`self.ArrowStaticMesh`) (`KismetMathLibrary.MakeVector` 0.0 0.0 (* (`GameplayStatics.GetWorldDeltaSeconds`) (`self.ArrowMovementSpeed`))) false false)
    (else
      (`SceneComponent.K2_AddLocalOffset` (`self.ArrowStaticMesh`) (`KismetMathLibrary.MakeVector` 0.0 0.0 (* (`GameplayStatics.GetWorldDeltaSeconds`) (`self.ArrowMovementSpeed`) -1.0)) false false)))
  (set `self.ArrowMovementCounter` (+ (`self.ArrowMovementCounter`) (* (`GameplayStatics.GetWorldDeltaSeconds`) (`self.ArrowMovementSpeed`))))
  (if (> (`self.ArrowMovementCounter`) (`self.ArrowMovementMax`))
    ;[1 1 1] Invert movement direction
    (set `self.MoveArrowUp` (not (`self.MoveArrowUp`)))
    (set `self.ArrowMovementCounter` 0.0)))

(event `self.BoxCollision.OnComponentBeginOverlap`
  (params (OverlappedComponent :type "PrimitiveComponent Object Reference") (OtherActor :type "Actor Object Reference") (OtherComp :type "PrimitiveComponent Object Reference") (OtherBodyIndex :type Integer) (bFromSweep :type Boolean) (SweepResult :type "HitResult Structure (by ref)"))
  (bind _asjigsaw_level_piece_movable_block (cast `/Game/Blueprints/Other/JigsawLevelPieceMovableBlock` OtherActor))
  (if (== (`self.JigsawPieceIndex`) (`/Game/Blueprints/Other/JigsawLevelPieceMovableBlock.JigsawPieceIndex` _asjigsaw_level_piece_movable_block))
    (set `self.JigsawPieceHasBeenPlacedCorrectly` true)
    (bind _returnvalue (`GameplayStatics.GetActorOfClass` "/Game/Blueprints/Other/JigsawPuzzleLevelBarrier.JigsawPuzzleLevelBarrier_C" :!label _label))
    (`/Game/Blueprints/Other/JigsawPuzzleLevelBarrier.CheckJigsawPuzzleStatus` _returnvalue)))

(event `self.BoxCollision.OnComponentEndOverlap`
  (params (OverlappedComponent :type "PrimitiveComponent Object Reference") (OtherActor :type "Actor Object Reference") (OtherComp :type "PrimitiveComponent Object Reference") (OtherBodyIndex :type Integer))
  (set `self.JigsawPieceHasBeenPlacedCorrectly` false)
  (goto _label))

(fn `UserConstructionScript`)