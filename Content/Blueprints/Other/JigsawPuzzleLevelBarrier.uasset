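; A level barrier actor that blocks progress until every piece of a jigsaw puzzle is placed correctly.
; CheckJigsawPuzzleStatus scans all JigsawLevelPieceBase actors in the level and calls DestroyLevelBarrier only if each is flagged as correctly placed.
; DestroyLevelBarrier shows the puzzle complete banner on the player character's HUD, waits briefly, then destroys the barrier.
; BeginPlay and Tick are unused, and nothing in this Blueprint calls the check itself.
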(event `DestroyLevelBarrier`
  (bind _asthird_person_character (cast `/Game/Blueprints/ThirdPersonCharacter` (`GameplayStatics.GetPlayerCharacter` 0)))
  (`/Game/Widgets/HUD.ShowPuzzleCompleteBanner` (`/Game/Blueprints/ThirdPersonCharacter.HUD` _asthird_person_character))
  (`KismetSystemLibrary.Delay` 1.0)
  (`self.K2_DestroyActor`))

(fn `CheckJigsawPuzzleStatus`
  (locals (AllPiecesHaveBeenPlacedCorrectly :type Boolean))
  (set `local.AllPiecesHaveBeenPlacedCorrectly` true)
  (bind _outactors (`GameplayStatics.GetAllActorsOfClass` "/Game/Blueprints/Other/JigsawLevelPieceBase.JigsawLevelPieceBase_C"))
  (for _array_element _outactors
    (bind _asjigsaw_level_piece_base (cast `/Game/Blueprints/Other/JigsawLevelPieceBase` _array_element))
    (if (not (`/Game/Blueprints/Other/JigsawLevelPieceBase.JigsawPieceHasBeenPlacedCorrectly` _asjigsaw_level_piece_base))
      (set `local.AllPiecesHaveBeenPlacedCorrectly` false)))
  (if (`local.AllPiecesHaveBeenPlacedCorrectly`)
    (`self.DestroyLevelBarrier`)))

(fn `UserConstructionScript`)