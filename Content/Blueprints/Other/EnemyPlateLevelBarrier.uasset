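; EnemyPlateLevelBarrier is a level barrier that removes itself once every EnemyPlate in the level has been hit by the player.
; CheckEnemyPlatesStatus scans all EnemyPlate actors for their HitByPlayer flag and, if none remain unhit, calls the DestroyLevelBarrier event to destroy the actor.
; Nothing in this Blueprint polls or triggers that check itself, as BeginPlay and Tick are unused.
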(event `DestroyLevelBarrier`
  (`self.K2_DestroyActor`))

(fn `CheckEnemyPlatesStatus`
  (locals (AllEnemyPlatesHaveBeenHit :type Boolean))
  (set `local.AllEnemyPlatesHaveBeenHit` true)
  (bind _outactors (`GameplayStatics.GetAllActorsOfClass` "/Game/Blueprints/Other/EnemyPlate.EnemyPlate_C"))
  (for _array_element _outactors
    (bind _asenemy_plate (cast `/Game/Blueprints/Other/EnemyPlate` _array_element))
    (if (not (`/Game/Blueprints/Other/EnemyPlate.HitByPlayer` _asenemy_plate))
      (set `local.AllEnemyPlatesHaveBeenHit` false)))
  (if (`local.AllEnemyPlatesHaveBeenHit`)
    (`self.DestroyLevelBarrier`)))

(fn `UserConstructionScript`)