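; EnemyPlate is an actor the player hits once to register it as struck.
; On the first hit by a ThirdPersonCharacter, it sets a one-time flag, increments the game mode's level plate count and updates the HUD with it.
; It then desaturates its mesh through a dynamic material instance and has the EnemyPlateLevelBarrier check the status of all plates.
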(event `self.ReceiveHit`
  (params (MyComp :type "PrimitiveComponent Object Reference") (Other :type "Actor Object Reference") (OtherComp :type "PrimitiveComponent Object Reference") (bSelfMoved :type Boolean) (HitLocation :type "Vector Structure") (HitNormal :type "Vector Structure") (NormalImpulse :type "Vector Structure") (Hit :type "HitResult Structure (by ref)"))
  (if (not (`self.HitByPlayer`))
    (bind _asthird_person_character (cast `/Game/Blueprints/ThirdPersonCharacter` Other))
    (set `self.HitByPlayer` true)
    (bind _currenttotalenemyplateshit (`/Game/Blueprints/ThirdPersonGameMode.AddTotalLevelEnemyPlatesHit` (`/Game/Blueprints/ThirdPersonCharacter.ThirdPersonGameMode` _asthird_person_character) 1))
    (`/Game/Widgets/HUD.UpdateTotalLevelEnemyPlatesHit` (`/Game/Blueprints/ThirdPersonCharacter.HUD` _asthird_person_character) _currenttotalenemyplateshit)
    (bind _returnvalue (`PrimitiveComponent.CreateDynamicMaterialInstance` (`self.EnemyPlateStaticMesh`) 0 "/Game/Materials/MaterialInstances/EnemyPlateMaterialInst.EnemyPlateMaterialInst" "None"))
    (`MaterialInstanceDynamic.SetScalarParameterValue` _returnvalue "DesaturationFraction" 1.0)
    (bind _returnvalue_2 (`GameplayStatics.GetActorOfClass` "/Game/Blueprints/Other/EnemyPlateLevelBarrier.EnemyPlateLevelBarrier_C"))
    (`/Game/Blueprints/Other/EnemyPlateLevelBarrier.CheckEnemyPlatesStatus` _returnvalue_2)))

(fn `UserConstructionScript`)