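; A jigsaw puzzle piece block that the player moves around the level by standing in its directional arrow meshes, with its picture mesh set at construction.
; Arrow overlaps by the ThirdPersonCharacter toggle four direction flags, which Tick turns into frame-rate-independent local offsets.
; Each tick also fakes gravity by snapping the block to a downward trace hit; landing on LevelAbsoluteFloor triggers game over through damage based on the player's initial HP.
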(event `self.ReceiveTick`
  (params (DeltaSeconds :type "Float (single-precision)"))
  (`self.SimulateGravityFall`)
  (`|ExecutionSequence`
    (:`then_0`
      (if (`self.MoveForward`)
        (`self.K2_AddActorLocalOffset` (`KismetMathLibrary.MakeVector` (* (`self.BlockMovementSpeed`) (`GameplayStatics.GetWorldDeltaSeconds`) -1.0)))))
    (:`then_1`
      (if (`self.MoveBackwards`)
        (`self.K2_AddActorLocalOffset` (`KismetMathLibrary.MakeVector` (* (`self.BlockMovementSpeed`) (`GameplayStatics.GetWorldDeltaSeconds`))))))
    (:`then_2`
      (if (`self.MoveLeft`)
        (`self.K2_AddActorLocalOffset` (`KismetMathLibrary.MakeVector` 0.0 (* (`self.BlockMovementSpeed`) (`GameplayStatics.GetWorldDeltaSeconds`))))))
    (:`then_3`
      (if (`self.MoveRight`)
        (`self.K2_AddActorLocalOffset` (`KismetMathLibrary.MakeVector` 0.0 (* (`self.BlockMovementSpeed`) (`GameplayStatics.GetWorldDeltaSeconds`) -1.0)))))))

(event `self.ForwardArrowStaticMesh.OnComponentBeginOverlap`
  (params (OverlappedComponent :type "PrimitiveComponent Object Reference") (OtherActor :type "Actor Object Reference") (OtherComp :type "PrimitiveComponent Object Reference") (OtherBodyIndex :type Integer) (bFromSweep :type Boolean) (SweepResult :type "HitResult Structure (by ref)"))
  ;[1 1 1] Forward arrow events
  (cast `/Game/Blueprints/ThirdPersonCharacter` OtherActor)
  (set `self.MoveForward` true))

(event `self.ForwardArrowStaticMesh.OnComponentEndOverlap`
  (params (OverlappedComponent :type "PrimitiveComponent Object Reference") (OtherActor :type "Actor Object Reference") (OtherComp :type "PrimitiveComponent Object Reference") (OtherBodyIndex :type Integer))
  ;[1 1 1] Forward arrow events
  (cast `/Game/Blueprints/ThirdPersonCharacter` OtherActor)
  (set `self.MoveForward` false))

(event `self.BackwardsArrowStaticMesh.OnComponentBeginOverlap`
  (params (OverlappedComponent :type "PrimitiveComponent Object Reference") (OtherActor :type "Actor Object Reference") (OtherComp :type "PrimitiveComponent Object Reference") (OtherBodyIndex :type Integer) (bFromSweep :type Boolean) (SweepResult :type "HitResult Structure (by ref)"))
  ;[1 1 1] Backwards arrow events
  (cast `/Game/Blueprints/ThirdPersonCharacter` OtherActor)
  (set `self.MoveBackwards` true))

(event `self.BackwardsArrowStaticMesh.OnComponentEndOverlap`
  (params (OverlappedComponent :type "PrimitiveComponent Object Reference") (OtherActor :type "Actor Object Reference") (OtherComp :type "PrimitiveComponent Object Reference") (OtherBodyIndex :type Integer))
  ;[1 1 1] Backwards arrow events
  (cast `/Game/Blueprints/ThirdPersonCharacter` OtherActor)
  (set `self.MoveBackwards` false))

(event `self.LeftArrowStaticMesh.OnComponentBeginOverlap`
  (params (OverlappedComponent :type "PrimitiveComponent Object Reference") (OtherActor :type "Actor Object Reference") (OtherComp :type "PrimitiveComponent Object Reference") (OtherBodyIndex :type Integer) (bFromSweep :type Boolean) (SweepResult :type "HitResult Structure (by ref)"))
  ;[1 1 1] Left arrow events
  (cast `/Game/Blueprints/ThirdPersonCharacter` OtherActor)
  (set `self.MoveLeft` true))

(event `self.LeftArrowStaticMesh.OnComponentEndOverlap`
  (params (OverlappedComponent :type "PrimitiveComponent Object Reference") (OtherActor :type "Actor Object Reference") (OtherComp :type "PrimitiveComponent Object Reference") (OtherBodyIndex :type Integer))
  ;[1 1 1] Left arrow events
  (cast `/Game/Blueprints/ThirdPersonCharacter` OtherActor)
  (set `self.MoveLeft` false))

(event `self.RightArrowStaticMesh.OnComponentBeginOverlap`
  (params (OverlappedComponent :type "PrimitiveComponent Object Reference") (OtherActor :type "Actor Object Reference") (OtherComp :type "PrimitiveComponent Object Reference") (OtherBodyIndex :type Integer) (bFromSweep :type Boolean) (SweepResult :type "HitResult Structure (by ref)"))
  ;[1 1 1] Right arrow events
  (cast `/Game/Blueprints/ThirdPersonCharacter` OtherActor)
  (set `self.MoveRight` true))

(event `self.RightArrowStaticMesh.OnComponentEndOverlap`
  (params (OverlappedComponent :type "PrimitiveComponent Object Reference") (OtherActor :type "Actor Object Reference") (OtherComp :type "PrimitiveComponent Object Reference") (OtherBodyIndex :type Integer))
  ;[1 1 1] Right arrow events
  (cast `/Game/Blueprints/ThirdPersonCharacter` OtherActor)
  (set `self.MoveRight` false))

(fn `SimulateGravityFall`
  (locals (AllObjectTypes :type "Array of EObjectTypeQuery Enum"))
  (bind (_returnvalue_x _returnvalue_y _returnvalue_z) (`KismetMathLibrary.BreakVector` (`self.K2_GetActorLocation`)))
  (bind (_returnvalue_x_2 _returnvalue_y_2) (`KismetMathLibrary.BreakVector` (`self.K2_GetActorLocation`)))
  (bind (_outhit _returnvalue) (`KismetSystemLibrary.LineTraceSingleForObjects` (`self.K2_GetActorLocation`) (`KismetMathLibrary.MakeVector` _returnvalue_x _returnvalue_y (- _returnvalue_z 10000.0)) (`local.AllObjectTypes`)))
  (if _returnvalue
    (`self.K2_SetActorLocation` (`KismetMathLibrary.MakeVector` _returnvalue_x_2 _returnvalue_y_2 (.z (`.Location` (`GameplayStatics.BreakHitResult` _outhit)))))
    (cast `/Game/Blueprints/Other/LevelAbsoluteFloor` (`.HitActor` (`GameplayStatics.BreakHitResult` _outhit)))
    ;[1 1 1] Game Over
    (bind _asthird_person_character (cast `/Game/Blueprints/ThirdPersonCharacter` (`GameplayStatics.GetPlayerCharacter` 0)))
    (`/Game/Blueprints/ThirdPersonCharacter.TakeDamage` _asthird_person_character (* (`/Game/Blueprints/ThirdPersonCharacter.HPInitialCache` _asthird_person_character) -1))))

(fn `UserConstructionScript`
  (`StaticMeshComponent.SetStaticMesh` (`self.PiecePictureStaticMesh`) (`self.PiecePicture`)))