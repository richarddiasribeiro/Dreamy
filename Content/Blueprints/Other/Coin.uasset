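; Coin actor that spins continuously and plays a short vanish animation when its DestroySelf event is called.
; Tick yaws it by RotationSpeed and, once ThrowUpwards is set, also moves it along its local Z axis, both scaled by delta time.
; DestroySelf turns off overlap events, sets the sphere to physics-only collision, speeds up the spin, starts the rise, then destroys the actor after a brief delay.
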(event `self.ReceiveTick`
  (params (DeltaSeconds :type "Float (single-precision)"))
  ;[1 1 1] Rotate
  (`self.K2_AddActorLocalRotation` (`KismetMathLibrary.MakeRotator` 0.0 0.0 (* (`GameplayStatics.GetWorldDeltaSeconds`) (`self.RotationSpeed`))))
  (if (`self.ThrowUpwards`)
    ;[1 1 1] Throw upwards
    (`self.K2_AddActorLocalOffset` (`KismetMathLibrary.MakeVector` 0.0 0.0 (* 250.0 (`GameplayStatics.GetWorldDeltaSeconds`))))))

(event `Destroy Self`
  (set `PrimitiveComponent.bGenerateOverlapEvents` false (`self.StaticMesh`))
  (set `PrimitiveComponent.bGenerateOverlapEvents` false (`self.Sphere`))
  (`PrimitiveComponent.SetCollisionEnabled` (`self.Sphere`) "PhysicsOnly")
  (set `self.RotationSpeed` 1800.0)
  (set `self.ThrowUpwards` true)
  (`KismetSystemLibrary.Delay` 0.25)
  (`self.K2_DestroyActor`))

(fn `UserConstructionScript`)