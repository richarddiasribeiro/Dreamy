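; RoadTool is a construction-script tool that lays a road mesh along an editable spline.
; It splits the spline length by DistanceBetween and adds a spline mesh component per segment with a configurable mesh, material and cross-section scale.
; Segment tangents are clamped to the spacing, and nothing is built when the spacing is under 100 units to cap the component count.
; The event graph has no active logic.
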(fn `UserConstructionScript`
  ;[1 1 1] Limit the spline from creating too many segments
  (if (>= (`self.DistanceBetween`) 100.0)
    (for _index (range (+ (`KismetMathLibrary.FTrunc` (/ (`SplineComponent.GetSplineLength` (`self.Spline`)) (`self.DistanceBetween`))) 1))
      (bind _returnvalue (`AddComponent|NODE_AddSplineMeshComponent-0`))
      (`StaticMeshComponent.SetStaticMesh` _returnvalue (`self.StaticMesh`))
      (`SplineMeshComponent.SetStartAndEnd` _returnvalue (`SplineComponent.GetLocationAtDistanceAlongSpline` (`self.Spline`) (* _index (`self.DistanceBetween`)) "Local") (`KismetMathLibrary.ClampVectorSize` (`SplineComponent.GetTangentAtDistanceAlongSpline` (`self.Spline`) (* _index (`self.DistanceBetween`)) "Local") 0.0 (`self.DistanceBetween`)) (`SplineComponent.GetLocationAtDistanceAlongSpline` (`self.Spline`) (* (+ _index 1) (`self.DistanceBetween`)) "Local") (`KismetMathLibrary.ClampVectorSize` (`SplineComponent.GetTangentAtDistanceAlongSpline` (`self.Spline`) (* (+ _index 1) (`self.DistanceBetween`)) "Local") 0.0 (`self.DistanceBetween`)) true)
      (`SplineMeshComponent.SetStartScale` _returnvalue (`KismetMathLibrary.MakeVector2D` (`self.ScaleInX`) (`self.ScaleInY`)) true)
      (`SplineMeshComponent.SetEndScale` _returnvalue (`KismetMathLibrary.MakeVector2D` (`self.ScaleInX`) (`self.ScaleInY`)) true)
      (`PrimitiveComponent.SetMaterial` _returnvalue 0 (`self.Material`)))))