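; A car actor that travels a scripted, timed route by itself, then climbs and finally falls.
; Tick accumulates a timer and moves the actor forward by Speed, making four quarter turns at fixed intervals, two one way and two back.
; A boolean array makes each turn fire once.
; After the turns it adds upward movement, until the last time threshold stops the climb and enables physics on the mesh.
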(event `self.ReceiveTick`
  (params (DeltaSeconds :type "Float (single-precision)"))
  (set `self.Timer` (+ DeltaSeconds (`self.Timer`)))
  ;[1 1 1] Make the car fall after a certain number of seconds
  (if (> (`self.Timer`) 120.0)
    (`PrimitiveComponent.SetSimulatePhysics` (`self.StaticMesh`) true)
    (`KismetArrayLibrary.Array_Set` (`self.ChangesDone`) 4 true))
  ;[1 1 1] Check for changes in the direction
  (if (and (> (`self.Timer`) 20.0) (not (`|GetArrayItem` (`self.ChangesDone`))))
    (`self.K2_AddActorLocalRotation` (struct :`Yaw` 90.0))
    (`KismetArrayLibrary.Array_Set` (`self.ChangesDone`) 0 true)
    (elif (and (> (`self.Timer`) 40.0) (not (`|GetArrayItem` (`self.ChangesDone`) 1)))
      (`self.K2_AddActorLocalRotation` (struct :`Yaw` 90.0))
      (`KismetArrayLibrary.Array_Set` (`self.ChangesDone`) 1 true)
      (elif (and (> (`self.Timer`) 60.0) (not (`|GetArrayItem` (`self.ChangesDone`) 2)))
        (`self.K2_AddActorLocalRotation` (struct :`Yaw` -90.0))
        (`KismetArrayLibrary.Array_Set` (`self.ChangesDone`) 2 true)
        (elif (and (> (`self.Timer`) 80.0) (not (`|GetArrayItem` (`self.ChangesDone`) 3)))
          (`self.K2_AddActorLocalRotation` (struct :`Yaw` -90.0))
          (`KismetArrayLibrary.Array_Set` (`self.ChangesDone`) 3 true)
          (elif (and (> (`self.Timer`) 100.0) (not (`|GetArrayItem` (`self.ChangesDone`) 4)))
            (`self.K2_AddActorLocalOffset` (`KismetMathLibrary.MakeVector` 0.0 0.0 (* (`self.Speed`) (`GameplayStatics.GetWorldDeltaSeconds`)))))))))
  ;[1 1 1] Move forward
  (`self.K2_AddActorLocalOffset` (`KismetMathLibrary.MakeVector` (* (`self.Speed`) (`GameplayStatics.GetWorldDeltaSeconds`)))))

(fn `UserConstructionScript`)