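; Barricade is a player skill actor that kills enemies on contact and removes itself after 60 seconds.
; When an Enemy overlaps its static mesh, it moves its death particle system to the enemy, scales particle count by that enemy's multiplier and activates it.
; It then hands the kill to the player's ThirdPersonCharacter through DestroyEnemy and destroys itself two seconds later.
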(event `self.ReceiveBeginPlay`
  (`KismetSystemLibrary.Delay` 60.0)
  (`self.K2_DestroyActor`))

(event `self.BarricadeStaticMeshComponent.OnComponentBeginOverlap`
  (params (OverlappedComponent :type "PrimitiveComponent Object Reference") (OtherActor :type "Actor Object Reference") (OtherComp :type "PrimitiveComponent Object Reference") (OtherBodyIndex :type Integer) (bFromSweep :type Boolean) (SweepResult :type "HitResult Structure (by ref)"))
  (bind _asenemy (cast `/Game/Blueprints/Enemies/Enemy` OtherActor))
  (`self.DestroyEnemyParticleSpawn` _asenemy (`self.K2_GetActorLocation` _asenemy))
  (bind _asthird_person_character (cast `/Game/Blueprints/ThirdPersonCharacter` (`GameplayStatics.GetPlayerCharacter` 0)))
  (`/Game/Blueprints/ThirdPersonCharacter.DestroyEnemy` _asthird_person_character _asenemy)
  (`KismetSystemLibrary.Delay` 2.0)
  (`self.K2_DestroyActor`))

(fn `DestroyEnemyParticleSpawn`
  (params (enemy :type "/Game/Blueprints/Enemies/Enemy Object Reference") (location :type "Vector Structure"))
  (bind _enemydeathparticlesystem (`self.EnemyDeathParticleSystem`))
  (`FXSystemComponent.SetIntParameter` _enemydeathparticlesystem "DeathParticleCountMultiplier" (`/Game/Blueprints/Enemies/Enemy.DeathParticleCountMultiplier` enemy))
  (`SceneComponent.K2_SetWorldLocation` _enemydeathparticlesystem location false false)
  (`ActorComponent.Activate` _enemydeathparticlesystem true))

(fn `UserConstructionScript`)