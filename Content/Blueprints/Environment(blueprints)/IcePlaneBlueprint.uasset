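; IcePlaneBlueprint is an ice surface actor that makes the ThirdPersonCharacter slide and move faster while overlapping it.
; On overlap begin it zeroes the character movement's braking friction factor and raises max walk speed.
; On overlap end it writes back fixed friction and speed values rather than saved ones, with both speeds scaled by the character's SpeedInitialCache.
; Debug strings print on entering and leaving.
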(event `self.ReceiveActorBeginOverlap`
  (params (OtherActor :type "Actor Object Reference"))
  (bind _asthird_person_character (cast `/Game/Blueprints/ThirdPersonCharacter` OtherActor))
  (bind _charactermovement (`Character.CharacterMovement` _asthird_person_character))
  ;[1 1 1] Replace player's friction and speed's default values
  ;;[1 1 1] Friction
  (set `CharacterMovementComponent.BrakingFrictionFactor` 0.0 _charactermovement)
  ;;[1 1 1] Speed
  (set `CharacterMovementComponent.MaxWalkSpeed` (* 1300.0 (`/Game/Blueprints/ThirdPersonCharacter.SpeedInitialCache` _asthird_person_character)) _charactermovement)
  (`KismetSystemLibrary.PrintString` "Slippery"))

(event `self.ReceiveActorEndOverlap`
  (params (OtherActor :type "Actor Object Reference"))
  (bind _asthird_person_character (cast `/Game/Blueprints/ThirdPersonCharacter` OtherActor))
  (bind _charactermovement (`Character.CharacterMovement` _asthird_person_character))
  ;[1 1 1] Replace player's friction and speed's default values
  ;;[1 1 1] Friction
  (set `CharacterMovementComponent.BrakingFrictionFactor` 2.0 _charactermovement)
  ;;[1 1 1] Speed
  (set `CharacterMovementComponent.MaxWalkSpeed` (* 725.0 (`/Game/Blueprints/ThirdPersonCharacter.SpeedInitialCache` _asthird_person_character)) _charactermovement)
  (`KismetSystemLibrary.PrintString` "Not slippery"))

(fn `UserConstructionScript`)