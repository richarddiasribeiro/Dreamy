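; MovingSandCube is an environment actor that moves back and forth along a local-space vector.
; Each Tick applies MovementVector scaled by delta time, negated on the return leg, as a local offset without sweep.
; An accumulated timer flips the MoveForward flag and resets on reaching MovementTimeMax, so reversal depends on elapsed time rather than distance or endpoints.
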(event `self.ReceiveTick`
  (params (DeltaSeconds :type "Float (single-precision)"))
  (if (`self.MoveForward`)
    (`self.K2_AddActorLocalOffset` (* (`self.MovementVector`) DeltaSeconds))
    (else
      (`self.K2_AddActorLocalOffset` (* (* (`self.MovementVector`) DeltaSeconds) -1.0))))
  (set `self.MovementTimeCounter` (+ (`self.MovementTimeCounter`) DeltaSeconds))
  (if (>= (`self.MovementTimeCounter`) (`self.MovementTimeMax`))
    (set `self.MoveForward` (not (`self.MoveForward`)))
    (set `self.MovementTimeCounter` 0.0)))

(fn `UserConstructionScript`)