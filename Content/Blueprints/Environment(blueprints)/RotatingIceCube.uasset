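; Environment actor for a rotating ice cube: a mesh that circles a pivot, driven by per-axis rotation and offset variables.
; BeginPlay shifts the StaticMesh locally by InitialOffset, away from its starting position.
; Each Tick, the Scene component rotates in world space by Rotation scaled by delta time.
; The mesh receives the negated rotation locally, countering the spin so it travels around the pivot while largely keeping its orientation.
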(event `self.ReceiveBeginPlay`
  (bind (_initialoffset_x _initialoffset_y _initialoffset_z) (`KismetMathLibrary.BreakVector` (`self.InitialOffset`)))
  (`SceneComponent.K2_AddLocalOffset` (`self.StaticMesh`) (`KismetMathLibrary.MakeVector` _initialoffset_x _initialoffset_y _initialoffset_z) false false))

(event `self.ReceiveTick`
  (params (DeltaSeconds :type "Float (single-precision)"))
  (bind (_returnvalue_x _returnvalue_y _returnvalue_z) (`KismetMathLibrary.BreakVector` (* (`self.Rotation`) DeltaSeconds)))
  (bind (_returnvalue_x_2 _returnvalue_y_2 _returnvalue_z_2) (`KismetMathLibrary.BreakVector` (* (`self.Rotation`) DeltaSeconds)))
  (bind (_returnvalue_x_3 _returnvalue_y_3 _returnvalue_z_3) (`KismetMathLibrary.BreakVector` (* (`KismetMathLibrary.MakeVector` _returnvalue_x _returnvalue_y _returnvalue_z) -1.0)))
  (`SceneComponent.K2_AddWorldRotation` (`self.Scene`) (`KismetMathLibrary.MakeRotator` _returnvalue_x_2 _returnvalue_y_2 _returnvalue_z_2) false false)
  (`SceneComponent.K2_AddLocalRotation` (`self.StaticMesh`) (`KismetMathLibrary.MakeRotator` _returnvalue_x_3 _returnvalue_y_3 _returnvalue_z_3) false false))

(fn `UserConstructionScript`)