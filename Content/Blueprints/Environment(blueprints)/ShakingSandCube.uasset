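; Sand cube environment hazard that shakes until hit, then falls away.
; Tick applies a small random rotation to the static mesh until the HitThePlayer flag is set.
; Any component hit on the mesh levels it and sets that flag, with no check on what struck it.
; After ShakingGroundReactionTime the mesh starts simulating physics, and the actor destroys itself ten seconds later.
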(event `self.ReceiveTick`
  (params (DeltaSeconds :type "Float (single-precision)"))
  (if (not (`self.HitThePlayer`))
    (`SceneComponent.K2_SetRelativeRotation` (`self.StaticMesh`) (`KismetMathLibrary.MakeRotator` (`KismetMathLibrary.RandomFloatInRange` -4.5 4.5) (`KismetMathLibrary.RandomFloatInRange` -4.5 4.5) (`KismetMathLibrary.RandomFloatInRange` -4.5 4.5)) false false)
    (`KismetSystemLibrary.Delay` 0.5)))

(event `self.StaticMesh.OnComponentHit`
  (params (HitComponent :type "PrimitiveComponent Object Reference") (OtherActor :type "Actor Object Reference") (OtherComp :type "PrimitiveComponent Object Reference") (NormalImpulse :type "Vector Structure") (Hit :type "HitResult Structure (by ref)"))
  ;[1 1 1] Stop shaking
  (`SceneComponent.K2_SetRelativeRotation` :`self` (`self.StaticMesh`))
  (set `self.HitThePlayer` true)
  (`KismetSystemLibrary.Delay` (`self.ShakingGroundReactionTime`))
  ;[1 1 1] Start falling
  (`PrimitiveComponent.SetSimulatePhysics` (`self.StaticMesh`) true)
  (`KismetSystemLibrary.Delay` 10.0)
  ;[1 1 1] Free from memory after some time
  (`self.K2_DestroyActor`))

(fn `UserConstructionScript`)