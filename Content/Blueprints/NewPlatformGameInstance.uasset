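; Game instance that holds player progression, settings and cutscene flags, and persists them to a single save slot.
; SaveTheGame copies XP, skills, classes, levels, menu selections, vibration, camera and audio settings into a new SaveGameBlueprint1 and writes it to "Save1".
; LoadTheGame reads that slot and copies the values back, stopping silently if the cast fails.
; Both functions print a message on completion.
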(fn `LoadTheGame`
  (bind _returnvalue (`GameplayStatics.LoadGameFromSlot` "Save1"))
  (bind _assave_game_blueprint_1 (cast `/Game/Blueprints/SaveGameBlueprint1` _returnvalue))
  (set `self.PlayerXP` (`/Game/Blueprints/SaveGameBlueprint1.PlayerXP` _assave_game_blueprint_1))
  (set `self.SelectedClassArrayIndex` (`/Game/Blueprints/SaveGameBlueprint1.SelectedClassArrayIndex` _assave_game_blueprint_1))
  (set `self.PlayerSkills` (`/Game/Blueprints/SaveGameBlueprint1.PlayerSkills` _assave_game_blueprint_1))
  (set `self.PlayerSkillsInventory` (`/Game/Blueprints/SaveGameBlueprint1.PlayerSkillsInventory` _assave_game_blueprint_1))
  (set `self.Classes` (`/Game/Blueprints/SaveGameBlueprint1.Classes` _assave_game_blueprint_1))
  (set `self.Levels` (`/Game/Blueprints/SaveGameBlueprint1.Levels` _assave_game_blueprint_1))
  (set `self.PlayerAttackVibrationIntensity` (`/Game/Blueprints/SaveGameBlueprint1.PlayerAttackVibrationIntensity` _assave_game_blueprint_1))
  (set `self.PlayerAttackVibrationDuration` (`/Game/Blueprints/SaveGameBlueprint1.PlayerAttackVibrationDuration` _assave_game_blueprint_1))
  (set `self.EnemyAttackVibrationIntensity` (`/Game/Blueprints/SaveGameBlueprint1.EnemyAttackVibrationIntensity` _assave_game_blueprint_1))
  (set `self.EnemyAttackVibrationDuration` (`/Game/Blueprints/SaveGameBlueprint1.EnemyAttackVibrationDuration` _assave_game_blueprint_1))
  (set `self.CameraSensitivity` (`/Game/Blueprints/SaveGameBlueprint1.CameraSensitivity` _assave_game_blueprint_1))
  (set `self.SFX` (`/Game/Blueprints/SaveGameBlueprint1.SFX` _assave_game_blueprint_1))
  (set `self.Music` (`/Game/Blueprints/SaveGameBlueprint1.Music` _assave_game_blueprint_1))
  (set `self.HasSeenInitialCutscene` (`/Game/Blueprints/SaveGameBlueprint1.HasSeenInitialCutscene` _assave_game_blueprint_1))
  (set `self.HasSeenEndCutscene` (`/Game/Blueprints/SaveGameBlueprint1.HasSeenEndCutscene` _assave_game_blueprint_1))
  (set `self.SelectedSkillInTheMenuArrayIndex` (`/Game/Blueprints/SaveGameBlueprint1.SelectedSkillInTheMenuArrayIndex` _assave_game_blueprint_1))
  (set `self.SelectedClassInTheMenuArrayIndex` (`/Game/Blueprints/SaveGameBlueprint1.SelectedClassInTheMenuArrayIndex` _assave_game_blueprint_1))
  (`KismetSystemLibrary.PrintString` "Load complete"))

(fn `SaveTheGame`
  (bind _returnvalue (`GameplayStatics.CreateSaveGameObject` "/Game/Blueprints/SaveGameBlueprint1.SaveGameBlueprint1_C"))
  (set `/Game/Blueprints/SaveGameBlueprint1.PlayerXP` (`self.PlayerXP`) _returnvalue)
  (set `/Game/Blueprints/SaveGameBlueprint1.SelectedClassArrayIndex` (`self.SelectedClassArrayIndex`) _returnvalue)
  (set `/Game/Blueprints/SaveGameBlueprint1.PlayerSkills` (`self.PlayerSkills`) _returnvalue)
  (set `/Game/Blueprints/SaveGameBlueprint1.PlayerSkillsInventory` (`self.PlayerSkillsInventory`) _returnvalue)
  (set `/Game/Blueprints/SaveGameBlueprint1.Classes` (`self.Classes`) _returnvalue)
  (set `/Game/Blueprints/SaveGameBlueprint1.Levels` (`self.Levels`) _returnvalue)
  (set `/Game/Blueprints/SaveGameBlueprint1.PlayerAttackVibrationIntensity` (`self.PlayerAttackVibrationIntensity`) _returnvalue)
  (set `/Game/Blueprints/SaveGameBlueprint1.PlayerAttackVibrationDuration` (`self.PlayerAttackVibrationDuration`) _returnvalue)
  (set `/Game/Blueprints/SaveGameBlueprint1.EnemyAttackVibrationIntensity` (`self.EnemyAttackVibrationIntensity`) _returnvalue)
  (set `/Game/Blueprints/SaveGameBlueprint1.EnemyAttackVibrationDuration` (`self.EnemyAttackVibrationDuration`) _returnvalue)
  (set `/Game/Blueprints/SaveGameBlueprint1.CameraSensitivity` (`self.CameraSensitivity`) _returnvalue)
  (set `/Game/Blueprints/SaveGameBlueprint1.SFX` (`self.SFX`) _returnvalue)
  (set `/Game/Blueprints/SaveGameBlueprint1.Music` (`self.Music`) _returnvalue)
  (set `/Game/Blueprints/SaveGameBlueprint1.HasSeenInitialCutscene` (`self.HasSeenInitialCutscene`) _returnvalue)
  (set `/Game/Blueprints/SaveGameBlueprint1.HasSeenEndCutscene` (`self.HasSeenEndCutscene`) _returnvalue)
  (set `/Game/Blueprints/SaveGameBlueprint1.SelectedSkillInTheMenuArrayIndex` (`self.SelectedSkillInTheMenuArrayIndex`) _returnvalue)
  (set `/Game/Blueprints/SaveGameBlueprint1.SelectedClassInTheMenuArrayIndex` (`self.SelectedClassInTheMenuArrayIndex`) _returnvalue)
  (`GameplayStatics.SaveGameToSlot` _returnvalue "Save1")
  (`KismetSystemLibrary.PrintString` "Save complete"))